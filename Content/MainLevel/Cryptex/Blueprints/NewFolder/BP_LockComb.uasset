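; BP_LockComb is a four-tumbler combination lock that ends the game when solved.
; It can randomize its BP_LockTumbler child actors on BeginPlay, and its box overlap toggles UsingLock on the FirstPersonCharacter.
; A delayed Tick checks about once a second whether the concatenated tumbler numbers equal Combination.
; A match plays an unlock sound at the player once, then quits the game after a short delay.
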(event OnComponentBeginOverlap(Box)
  (params (OverlappedComponent :type Primitive%20Component%20Object%20Reference) (OtherActor :type Actor%20Object%20Reference) (OtherComp :type Primitive%20Component%20Object%20Reference) (OtherBodyIndex :type Integer) (bFromSweep :type Boolean) (SweepResult :type Hit%20Result%20Structure%20%28by%20ref%29))
  (bind _asfirst_person_character (Utilities|Casting|CastToFirstPersonCharacter OtherActor))
  (Variables|/Game/Templates/WISTerminals/Blueprints/Core/FirstPersonCharacter.FirstPersonCharacter_C|SetusingLock? _asfirst_person_character true))

(event OnComponentEndOverlap(Box)
  (params (OverlappedComponent :type Primitive%20Component%20Object%20Reference) (OtherActor :type Actor%20Object%20Reference) (OtherComp :type Primitive%20Component%20Object%20Reference) (OtherBodyIndex :type Integer))
  (bind _asfirst_person_character (Utilities|Casting|CastToFirstPersonCharacter OtherActor))
  (Variables|/Game/Templates/WISTerminals/Blueprints/Core/FirstPersonCharacter.FirstPersonCharacter_C|SetusingLock? _asfirst_person_character false))

(event EventTick
  (params (DeltaSeconds :type Float%20%28single-precision%29))
  ;[1 1 1] check for correct combination
  (Utilities|FlowControl|Delay 1.0)
  (bind _combomatch_ (CallFunction|CheckCombination))
  (if _combomatch_
    (Utilities|FlowControl|DoOnce false
      (:Completed
        (Audio|SpawnSoundatLocation "/Game/Sounds/Unlock_02.Unlock_02" (Transformation|GetActorLocation (Game|GetPlayerCharacter 0)) "0, 0, 0" 1.0 1.0 0.0 0 0)
        (Utilities|FlowControl|Delay 1.0)
        (Game|QuitGame 0 "Quit" false)))))

(event EventBeginPlay
  ;[1 1 1] randomize tumblrs?
  (if (Variables|Default|GetRandomizeTumRot?)
    (Default|RandomizeTumblr (.AsBP%20Lock%20Tumbler (Utilities|Casting|CastToBP_LockTumbler (Variables|/Script/Engine.ChildActorComponent|GetChildActor (Variables|Default|GetBP_LockTumbler1)))))
    (Default|RandomizeTumblr (.AsBP%20Lock%20Tumbler (Utilities|Casting|CastToBP_LockTumbler (Variables|/Script/Engine.ChildActorComponent|GetChildActor (Variables|Default|GetBP_LockTumbler2)))))
    (Default|RandomizeTumblr (.AsBP%20Lock%20Tumbler (Utilities|Casting|CastToBP_LockTumbler (Variables|/Script/Engine.ChildActorComponent|GetChildActor (Variables|Default|GetBP_LockTumbler3)))))
    (Default|RandomizeTumblr (.AsBP%20Lock%20Tumbler (Utilities|Casting|CastToBP_LockTumbler (Variables|/Script/Engine.ChildActorComponent|GetChildActor (Variables|Default|GetBP_LockTumbler4)))))))

(fn ConstructionScript)

(fn CheckCombination
  (return (Utilities|Enum|Equal(Enum) (Variables|Default|GetCombination) (Utilities|String|Append (Utilities|String|ToString(Integer) (Variables|/Game/Blueprints/NewFolder/BP_LockTumbler.BP_LockTumbler_C|GetTumblrNUmber (.AsBP%20Lock%20Tumbler (Utilities|Casting|CastToBP_LockTumbler (Variables|/Script/Engine.ChildActorComponent|GetChildActor (Variables|Default|GetBP_LockTumbler1)))))) (Utilities|String|ToString(Integer) (Variables|/Game/Blueprints/NewFolder/BP_LockTumbler.BP_LockTumbler_C|GetTumblrNUmber (.AsBP%20Lock%20Tumbler (Utilities|Casting|CastToBP_LockTumbler (Variables|/Script/Engine.ChildActorComponent|GetChildActor (Variables|Default|GetBP_LockTumbler2)))))) (Utilities|String|ToString(Integer) (Variables|/Game/Blueprints/NewFolder/BP_LockTumbler.BP_LockTumbler_C|GetTumblrNUmber (.AsBP%20Lock%20Tumbler (Utilities|Casting|CastToBP_LockTumbler (Variables|/Script/Engine.ChildActorComponent|GetChildActor (Variables|Default|GetBP_LockTumbler3)))))) (Utilities|String|ToString(Integer) (Variables|/Game/Blueprints/NewFolder/BP_LockTumbler.BP_LockTumbler_C|GetTumblrNUmber (.AsBP%20Lock%20Tumbler (Utilities|Casting|CastToBP_LockTumbler (Variables|/Script/Engine.ChildActorComponent|GetChildActor (Variables|Default|GetBP_LockTumbler4))))))))))