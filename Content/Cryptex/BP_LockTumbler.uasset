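; Rotating digit tumbler for a cryptex lock that can be spun forward or backward to show a number from 0 to 9.
; On BeginPlay it picks a random start rotation from an array and derives its digit.
; Interact and SpinBackwards each play a timeline that rolls the mesh, with DoOnce gates blocking repeat input until it finishes.
; NumberCheck then maps the truncated angle to the digit through a branch chain, and the rotation resets at a full turn.
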(event Custom|SpinBackwards
  ;[1 1 1] spin num
  (Utilities|FlowControl|DoOnce false
    (:Completed
      (bind _alpha (Timeline|Timeline_1 PlayFromStart)
        (:Update
          (Transformation|SetRelativeRotation (Variables|Default|GetTumbler%20mesh) (Math|Rotator|MakeRotator (- (Variables|Default|GetTumblr%20rotation) _alpha) 0.0 0.0) false false))
        (:Finished
          (Variables|Default|SetTumblr%20rotation (- (Variables|Default|GetTumblr%20rotation) _alpha))
          (CallFunction|NumberCheck)
          (CallFunction|ShowTumblNumber)
          (CallFunction|SpinBackReset)
          (if (<= (Variables|Default|GetTumblr%20rotation) -3.6e+02)
            (Variables|Default|SetTumblr%20rotation 0.0)))))))

(event Custom|SpinBackReset
  ;[1 1 1] spin num
  (Utilities|FlowControl|DoOnce false) ; enters at Reset
)

(event Custom|show%20tumbl%20number
  ;[1 1 1] show tumbl num
)

(event Custom|SpinTumblrReset
  ;[1 1 1] spin num
  (Utilities|FlowControl|DoOnce false) ; enters at Reset
)

(event EventInteract
  (params (Interactor :type Actor%20Object%20Reference))
  ;[1 1 1] spin num
  (Utilities|FlowControl|DoOnce false
    (:Completed
      (bind _alpha (Timeline|Timeline_0 PlayFromStart)
        (:Update
          (Transformation|SetRelativeRotation (Variables|Default|GetTumbler%20mesh) (Math|Rotator|MakeRotator (+ (Variables|Default|GetTumblr%20rotation) _alpha) 0.0 0.0) false false))
        (:Finished
          (Variables|Default|SetTumblr%20rotation (+ (Variables|Default|GetTumblr%20rotation) _alpha))
          (CallFunction|NumberCheck)
          (CallFunction|ShowTumblNumber)
          (CallFunction|SpinTumblrReset)
          (if (>= (Variables|Default|GetTumblr%20rotation) 3.6e+02)
            (Variables|Default|SetTumblr%20rotation 0.0)))))))

(event EventBeginPlay
  ;[1 1 1] beginplay
  (if true
    (CallFunction|RandomizeTumblr)))

(fn ConstructionScript)

(fn NumberCheck
  (if (== (Math|Float|Truncate (Variables|Default|GetTumblr%20rotation)) 0)
    (Variables|Default|SetTumblrNUmber 0)
    (elif (== (Math|Float|Truncate (Variables|Default|GetTumblr%20rotation)) 36)
      (Variables|Default|SetTumblrNUmber 1)
      (elif (== (Math|Float|Truncate (Variables|Default|GetTumblr%20rotation)) 72)
        (Variables|Default|SetTumblrNUmber 2)
        (elif (== (Math|Float|Truncate (Variables|Default|GetTumblr%20rotation)) 108)
          (Variables|Default|SetTumblrNUmber 3)
          (elif (== (Math|Float|Truncate (Variables|Default|GetTumblr%20rotation)) 144)
            (Variables|Default|SetTumblrNUmber 4)
            (elif (== (Math|Float|Truncate (Variables|Default|GetTumblr%20rotation)) 180)
              (Variables|Default|SetTumblrNUmber 5)
              (elif (== (Math|Float|Truncate (Variables|Default|GetTumblr%20rotation)) 216)
                (Variables|Default|SetTumblrNUmber 6)
                (elif (== (Math|Float|Truncate (Variables|Default|GetTumblr%20rotation)) 252)
                  (Variables|Default|SetTumblrNUmber 7)
                  (elif (== (Math|Float|Truncate (Variables|Default|GetTumblr%20rotation)) 288)
                    (Variables|Default|SetTumblrNUmber 8)
                    (elif (== (Math|Float|Truncate (Variables|Default|GetTumblr%20rotation)) 324)
                      (Variables|Default|SetTumblrNUmber 9)
                      (elif (== (Math|Float|Truncate (Variables|Default|GetTumblr%20rotation)) 360)
                        (Variables|Default|SetTumblrNUmber 0)
                        (elif (== (Math|Float|Truncate (Variables|Default|GetTumblr%20rotation)) -36)
                          (Variables|Default|SetTumblrNUmber 9)
                          (elif (== (Math|Float|Truncate (Variables|Default|GetTumblr%20rotation)) -72)
                            (Variables|Default|SetTumblrNUmber 8)
                            (elif (== (Math|Float|Truncate (Variables|Default|GetTumblr%20rotation)) -108)
                              (Variables|Default|SetTumblrNUmber 7)
                              (elif (== (Math|Float|Truncate (Variables|Default|GetTumblr%20rotation)) -144)
                                (Variables|Default|SetTumblrNUmber 6)
                                (elif (== (Math|Float|Truncate (Variables|Default|GetTumblr%20rotation)) -180)
                                  (Variables|Default|SetTumblrNUmber 5)
                                  (elif (== (Math|Float|Truncate (Variables|Default|GetTumblr%20rotation)) -216)
                                    (Variables|Default|SetTumblrNUmber 4)
                                    (elif (== (Math|Float|Truncate (Variables|Default|GetTumblr%20rotation)) -252)
                                      (Variables|Default|SetTumblrNUmber 3)
                                      (elif (== (Math|Float|Truncate (Variables|Default|GetTumblr%20rotation)) -288)
                                        (Variables|Default|SetTumblrNUmber 2)
                                        (elif (== (Math|Float|Truncate (Variables|Default|GetTumblr%20rotation)) -324)
                                          (Variables|Default|SetTumblrNUmber 1)
                                          (elif (== (Math|Float|Truncate (Variables|Default|GetTumblr%20rotation)) -360)
                                            (Variables|Default|SetTumblrNUmber 0)))))))))))))))))))))))

(fn RandomizeTumblr
  (bind _randomrotations (Variables|Default|GetRandomRotations))
  (bind _output_get (Variables|Default|SetTumblr%20rotation (Utilities|Array|Get(acopy) _randomrotations (Math|Random|RandomIntegerinRange 0 (- (Utilities|Array|Length _randomrotations) 1)))))
  (Transformation|SetRelativeRotation (Variables|Default|GetTumbler%20mesh) (Math|Rotator|MakeRotator _output_get 0.0 0.0) false false)
  (CallFunction|NumberCheck))