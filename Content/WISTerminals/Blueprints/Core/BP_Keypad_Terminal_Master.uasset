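; Master keypad terminal Blueprint that checks a four-digit code, optionally randomized, entered through a widget to unlock and activate linked objects.
; On start it links the widget to itself and disables the keypad if a linked object is already unlocked or active.
; Success records objects for saving and can turn the camera toward a target.
; Failure locks the keypad and shows a TerminalDoor1 widget once; the timed reset is disconnected.
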(event Custom|Compare
  (bind _terminalinterfaceinstance (Variables|Default|GetTerminalInterfaceInstance))
  ;[0 0.8745 1] Compare Codes
  (if (Utilities|Enum|Equal(Enum) (Variables|Default|GetUserInput) (Variables|Default|GetCode))
    ;[0.02821 0.5417 0.04296] Correct Code: Change Interface to Approved State and set Unlocked to True
    (Class|WidgetSwitcher|SetActiveWidgetIndex (Variables|/Game/WISTerminals/UserInterface/UI_Keypad_Terminal.UI_Keypad_Terminal_C|GetTerminalSwitch (Variables|Default|GetTerminalInterfaceInstance)) 2)
    (Variables|Default|SetUnlockedOrDisabled true)
    (CallFunction|UnlockandActivateObjects)
    (Audio|PlaySoundatLocation "/Game/WISTerminals/Sounds/Cues/SC_Terminal_Granted.SC_Terminal_Granted" (Transformation|GetWorldLocation (Variables|Default|GetWidget)) "0, 0, 0" 1.0 1.0 0.0 0 0 0)
    (if (Variables|Default|GetLookAtTargetWhenUnlocked?)
      (CallFunction|LookatTarget))
    ;[0.02821 0.5417 0.04296] Reset in case Door becomes locked again
    (Rendering|Components|TextRender|SetText (Variables|/Game/WISTerminals/UserInterface/UI_Keypad_Terminal.UI_Keypad_Terminal_C|GetNumber_01 _terminalinterfaceinstance) "")
    (Widget|SetIsEnabled (Variables|/Game/WISTerminals/UserInterface/UI_Keypad_Terminal.UI_Keypad_Terminal_C|GetButtonContainer _terminalinterfaceinstance) true)
    (else
      ;[0.5781 0.06536 0.05119] Wrong Code: Change Interface to Denied State
      (Variables|Default|SetUnlockedOrDisabled true)
      (Class|WidgetSwitcher|SetActiveWidgetIndex (Variables|/Game/WISTerminals/UserInterface/UI_Keypad_Terminal.UI_Keypad_Terminal_C|GetTerminalSwitch (Variables|Default|GetTerminalInterfaceInstance)) 1)
      (Audio|PlaySoundatLocation "/Game/WISTerminals/Sounds/Cues/SC_Terminal_Denied.SC_Terminal_Denied" (Transformation|GetWorldLocation (Variables|Default|GetWidget)) "0, 0, 0" 1.0 1.0 0.0 0 0 0)
      ;[1 1 1] OPEN BLOCKED DOOR (narukyn)
      (Utilities|FlowControl|DoOnce false
        (:Completed
          (bind _returnvalue (UserInterface|CreateWidget "/Game/Devs/Narukyn/InventorySystem/UI/TerminalDoor1.TerminalDoor1_C"))
          (UserInterface|Viewport|AddtoViewport _returnvalue 0))))))

(event Custom|LookAtTarget
  (bind _returnvalue (Game|GetPlayerController 0))
  (bind _returnvalue_2 (Game|GetPlayerController 0))
  ;[0 0.9451 1] Look at Target Point
  (Input|DisableInput (Game|Player|GetPlayerPawn 0) _returnvalue)
  (Variables|Default|SetLastControlRotation (Pawn|GetControlRotation _returnvalue :!class /Script/Engine.Controller))
  (bind _curve (Timeline|LookAtTargetTimeline PlayFromStart)
    (:Update
      (Pawn|SetControlRotation _returnvalue_2 (Math|Rotator|Lerp(Rotator) (Variables|Default|GetLastControlRotation) (Math|Rotator|FindLookatRotation (Camera|GetCameraLocation (Game|GetPlayerCameraManager 0)) (Transformation|GetActorLocation (Variables|Default|GetLookAtPoint))) _curve true)))
    (:Finished
      (Input|EnableInput (Game|Player|GetPlayerPawn 0) _returnvalue_2))))

(event Custom|DisableKeypad
  ;[0.02821 0.5417 0.04296] Enable or disable keypad
  (Class|WidgetSwitcher|SetActiveWidgetIndex (Variables|/Game/WISTerminals/UserInterface/UI_Keypad_Terminal.UI_Keypad_Terminal_C|GetTerminalSwitch (Variables|Default|GetTerminalInterfaceInstance)) 2)
  (Variables|Default|SetUnlockedOrDisabled true))

(event Custom|EnableKeypad
  ;[0.02821 0.5417 0.04296] Enable or disable keypad
  (Class|WidgetSwitcher|SetActiveWidgetIndex (Variables|/Game/WISTerminals/UserInterface/UI_Keypad_Terminal.UI_Keypad_Terminal_C|GetTerminalSwitch (Variables|Default|GetTerminalInterfaceInstance)))
  (Variables|Default|SetUnlockedOrDisabled false))

(event Custom|CreateRandomCode
  ;[0 0.8796 1] Create a Random Code at Runtime
  (if (Variables|Default|GetRandomCode?)
    (Variables|Default|SetCode (Utilities|Text|ToText(String) (Utilities|String|Append (Utilities|String|ToString(Integer) (Math|Random|RandomIntegerinRange 0 9)) (Utilities|String|ToString(Integer) (Math|Random|RandomIntegerinRange 0 9)) (Utilities|String|ToString(Integer) (Math|Random|RandomIntegerinRange 0 9)) (Utilities|String|ToString(Integer) (Math|Random|RandomIntegerinRange 0 9)))))))

(event Custom|InitializeKeypad
  ;[0 0.8745 1] Disable keypad if one or more locked objects have already been unlocked (by savegame)
  (bind _array_element (Utilities|Array|ForEachLoopwithBreak (Variables|Default|GetLockedObjects) :!label _label)
    (:LoopBody
      (if (or (Variables|/Game/WISTerminals/Blueprints/Core/BP_Master_LinkedObject.BP_Master_LinkedObject_C|GetActive _array_element) (not (Variables|/Game/WISTerminals/Blueprints/Core/BP_Master_LinkedObject.BP_Master_LinkedObject_C|GetLocked _array_element)))
        (CallFunction|DisableKeypad)
        (goto _label Break)
        (else
          (CallFunction|EnableKeypad))))))

(event Custom|UnlockAndActivateObjects
  ;[0 0.8745 1] Unlock Objects and Fire Activate Event / remember activated objects for saving
  (for _array_element (Variables|Default|GetLockedObjects)
    (Default|Activate _array_element)
    (Utilities|Array|AddUnique (Variables|/Game/WISTerminals/Blueprints/BP_TerminalController.BP_TerminalController_C|GetActivatedObjects (Variables|Default|GetTerminalController)) _array_element)))

(event EventBeginPlay
  ;[0 0.8745 1] Begin - Set self as Instance for respective UI_Terminal
  (|CallParentFunction)
  (bind _asui_keypad_terminal (Utilities|Casting|CastToUI_Keypad_Terminal (UserInterface|GetUserWidgetObject (Variables|Default|GetWidget))))
  (Variables|/Game/WISTerminals/UserInterface/UI_Keypad_Terminal.UI_Keypad_Terminal_C|SetTerminalInstance _asui_keypad_terminal self)
  (CallFunction|CreateRandomCode)
  (Utilities|FlowControl|Delay 0.3)
  (CallFunction|InitializeKeypad))

(fn ConstructionScript
  (Components|Timeline|SetPlayRate (Variables|Default|GetLookAtTargetTimeline) (Variables|Default|GetLookAtTimeRatio)))