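; Controller for interactive world-space terminals, driving a player-camera Widget Interaction Component with mouse or gamepad input.
; Each tick it detects front-facing terminal widgets, spawns a BP_Cursor at the hit point, and disables character turning while moving the pointer.
; Timelines align view and position to the terminal and optionally zoom FOV; sustained movement input releases focus.
; Save/load functions persist active linked objects and unlocked computer terminals to a save slot.
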(event Custom|LookAtDisplay
  (bind _returnvalue (Game|Player|GetPlayerPawn 0))
  (bind _returnvalue_2 (Game|GetPlayerController 0))
  (bind _activeterminal (Variables|Default|GetActiveTerminal))
  (bind _returnvalue_3 (Transformation|GetActorLocation _returnvalue))
  (bind _placementmarker (Variables|/Game/WISTerminals/Blueprints/Core/BP_Master_Terminal.BP_Master_Terminal_C|GetPlacementMarker _activeterminal))
  (bind _returnvalue_4 (Transformation|GetWorldLocation _placementmarker))
  ;[0 0.8796 1] Look at Center of Terminal Timeline Animation
  (bind _curve (Timeline|LookAtDisplayTimeline PlayFromStart)
    (:Update
      (Pawn|SetControlRotation _returnvalue_2 (Math|Rotator|Lerp(Rotator) (Pawn|GetControlRotation _returnvalue_2 :!class /Script/Engine.Controller) (Math|Rotator|FindLookatRotation (Camera|GetCameraLocation (Game|GetPlayerCameraManager 0)) (Transformation|GetWorldLocation (Variables|Default|GetActiveWidget))) _curve true))
      (Transformation|SetActorLocation _returnvalue (Math|Vector|Lerp(Vector) _returnvalue_3 (Math|Vector|MakeVector (.x _returnvalue_4) (.y _returnvalue_4) (.Z (Math|Vector|BreakVector _returnvalue_3))) _curve) true false)
      ;[0 0.8745 1] Stop Timeline when receiving movement Input close before Animation ends
      (if (>= (Components|Timeline|GetPlaybackPosition (Variables|Default|GetLookAtDisplayTimeline)) 0.4)
        (Variables|Default|SetInitialFocus false)
        (if (Utilities|ReceiveMovementInput)
          (Audio|Components|Audio|Stop (Variables|Default|GetLookAtDisplayTimeline)))))
    (:Finished
      (Variables|Default|SetInitialFocus false))))

(event Custom|SetupController
  ;[0 0.7373 1] Spawn and attach Widget Interaction Component to Player Camera
  (bind _returnvalue (AddComponent|AddWidgetInteractionComponent (Game|Player|GetPlayerPawn 0) true (Math|Transform|MakeTransform (Variables|/Script/Engine.SceneComponent|GetRelativeLocation (Variables|Default|GetPlayerCamera))) 0 0.0))
  (bind _output_get (Variables|Default|SetWidgetInteractionInstance _returnvalue))
  (Variables|/Script/UMG.WidgetInteractionComponent|SetInteractionDistance _output_get (Variables|Setup|GetInteractionDistance))
  (Transformation|AttachComponentToComponent _output_get (Variables|Default|GetPlayerCamera) "None" "SnapToTarget" "KeepRelative" "KeepRelative" true)
  ;[0 0.7373 1] Save Origin Camera Field of View
  (Variables|Default|SetOriginCameraFoV (Variables|/Script/Engine.CameraComponent|GetFieldOfView (Variables|Default|GetPlayerCamera))))

(event Custom|FieldOfViewZoom
  ;[0 0.8745 1] Camera Field of View Zoom
  (if (Variables|Default|GetZoomEnabled)
    (Variables|Default|SetStartFoV (Variables|/Script/Engine.CameraComponent|GetFieldOfView (Variables|Default|GetPlayerCamera)))
    (bind _curve (Timeline|FieldOfViewTimeline PlayFromStart)
      (:Update
        (Camera|SetFieldOfView (Variables|Default|GetPlayerCamera) (Math|Float|Lerp (Variables|Default|GetStartFoV) (Variables|Default|GetTargetFoV) _curve))))))

(event Custom|ControlCursorAndFocus
  (bind _widgetinteractioninstance (Variables|Default|GetWidgetInteractionInstance))
  (bind _returnvalue (Class|WidgetInteractionComponent|GetLastHitResult _widgetinteractioninstance))
  (bind (_bblockinghit _binitialoverlap _time _distance _location _impactpoint _normal _impactnormal _physmat _hitactor _hitcomponent) (Collision|BreakHitResult _returnvalue))
  ;[0 0.8745 1] Create a Cursor when hovering a focusable Widget, set Location to Hit Location and delete Cursor when Widget loses Focus
  (if (<= (Variables|Default|GetMovementInputHoldDownTimer) 2e+01)
    (|ShouldReceiveInput? _hitactor _hitcomponent
      (:true
        (Variables|Default|SetZoomEnabled (Variables|/Game/WISTerminals/Blueprints/Core/BP_Master_Terminal.BP_Master_Terminal_C|GetUseFieldOfViewZoom? (Variables|Default|GetActiveTerminal)))
        (Variables|Default|SetMoveComponent true)
        (Variables|Default|SetCharacterTurnInputEnabled? false)
        (if (== (Variables|Default|GetCursorInstance) 0)
          (bind _returnvalue_2 (Game|SpawnActorfromClass "/Game/WISTerminals/Blueprints/Core/BP_Cursor.BP_Cursor_C" (Math|Transform|MakeTransform _location (Math|Rotator|MakeRotfromY _normal)) "Undefined" 0 0))
          (Variables|Default|SetCursorInstance _returnvalue_2)
          (Utilities|FlowControl|DoOnce false :!label _label
            (:Completed
              (Variables|Default|SetInitialFocus true)
              (CallFunction|LookatDisplay)
              (Variables|Default|SetTargetFoV (Variables|/Game/WISTerminals/Blueprints/Core/BP_Master_Terminal.BP_Master_Terminal_C|GetFocusFieldOfView (Variables|Default|GetActiveTerminal)))
              (CallFunction|FieldOfViewZoom)
              (goto _label_3 Reset)))
          (else
            (Utilities|FlowControl|Sequence
              (:then_0
                (|KeepDisplayFocus)
                (goto _label Reset))
              (:then_1
                (Transformation|SetActorLocation (Variables|Default|GetCursorInstance) _location false false)
                (Transformation|AddRelativeLocation (Variables|Default|GetWidgetInteractionInstance) (Math|Vector|MakeVector 0.0 (+ (Variables|Default|GetXInput_Mouse) (* (Variables|Default|GetXInput_Gamepad) (Variables|Setup|GetGamepadSensitivity))) (* (+ (Variables|Default|GetYInput_Mouse) (* (Variables|Default|GetYInput_Gamepad) (Variables|Setup|GetGamepadSensitivity))) -1.0)) false false))))))
      (:false
        (if (not (Variables|Default|GetInitialFocus)) :!label _label_2 ; Don't stop initial focus animation
          (Audio|Components|Audio|Stop (Variables|Default|GetLookAtDisplayTimeline))
          (|ResetActiveTerminal)
          (|DeleteCursorAndClearCursorInstance)
          (Variables|Default|SetMoveComponent false)
          (Variables|Default|SetCharacterTurnInputEnabled? true)
          (Utilities|FlowControl|DoOnce false :!label _label_3
            (:Completed
              (Variables|Default|SetTargetFoV (Variables|Default|GetOriginCameraFoV))
              (CallFunction|FieldOfViewZoom))))))
    (else
      (goto _label_2))))

(event Custom|ResetLocation
  ;[0 0.8745 1] Reset Interaction Components relative Location
  (if (and (!= (Variables|Default|GetActiveWidget) 0) (not (Utilities|ReceiveMovementInput)))
    (|SingleLineTrace
      (:NoHit
        (Utilities|FlowControl|DoOnce false :!label _label
          (:Completed
            (Transformation|SetRelativeLocation (Variables|Default|GetWidgetInteractionInstance) "0, 0, 0" false false)
            ;[0 0.8745 1] Create a Cursor when hovering a focusable Widget, set Location to Hit Location and delete Cursor when Widget loses Focus
            (Utilities|FlowControl|DoOnce false) ; enters at Reset
          )))
      (:HitWidget
        (goto _label Reset)))))

(event Custom|UpdateTerminals
  ;[0 0.8745 1] Constantly check for terminals, create and move cursor and control input
  (|ShowHideCursor)
  (CallFunction|ControlCursorandFocus)
  (CallFunction|ResetLocation)
  (CallFunction|CountMovementInputHoldTime))

(event EventTick
  (params (DeltaSeconds :type Float%20%28single-precision%29))
  ;[0 0.8745 1] Constantly check for terminals, create and move cursor and control input
  (CallFunction|UpdateTerminals))

(event Input|ActionEvents|InputActionInteract
  (params (Key :type Key%20Structure))
  (bind _widgetinteractioninstance (Variables|Default|GetWidgetInteractionInstance))
  ;[0 0.8796 1] Receive Input
  (:Pressed
    (Class|WidgetInteractionComponent|PressPointerKey _widgetinteractioninstance "LeftMouseButton"))
  (:Released
    (Class|WidgetInteractionComponent|ReleasePointerKey _widgetinteractioninstance "LeftMouseButton")))

(event Input|MouseEvents|MouseWheelAxis
  (params (AxisValue :type Float%20%28single-precision%29))
  ;[0 0.8796 1] Receive Input
  (Class|WidgetInteractionComponent|ScrollWheel (Variables|Default|GetWidgetInteractionInstance) AxisValue))

(event Input|GamepadEvents|GamepadFaceButtonBottom
  (params (Key :type Key%20Structure))
  ;[0 0.8796 1] Receive Input
  (:Pressed
    (Class|WidgetInteractionComponent|PressandReleaseKey (Variables|Default|GetWidgetInteractionInstance) "LeftMouseButton")))

(event Input|GamepadEvents|GamepadDPadDown
  (params (Key :type Key%20Structure))
  ;[0 0.8796 1] Receive Input
  (:Pressed
    (Class|WidgetInteractionComponent|ScrollWheel (Variables|Default|GetWidgetInteractionInstance) -1.0)))

(event Input|GamepadEvents|GamepadDPadUp
  (params (Key :type Key%20Structure))
  ;[0 0.8796 1] Receive Input
  (:Pressed
    (Class|WidgetInteractionComponent|ScrollWheel (Variables|Default|GetWidgetInteractionInstance) 1.0)))

(fn ConstructionScript)

(fn ResetRelativeLocation
  (bind _activewidget (Variables|Default|GetActiveWidget))
  (if (not (== _activewidget 0))
    (if (not (Math|Rotator|Equal(Rotator) (Pawn|GetControlRotation (Game|GetPlayerController 0) :!class /Script/Engine.Controller) (Math|Rotator|FindLookatRotation (Camera|GetCameraLocation (Game|GetPlayerCameraManager 0)) (Transformation|GetWorldLocation _activewidget)) 2e+01))
      (Utilities|FlowControl|DoOnce false
        (:Completed
          (Transformation|ResetRelativeTransform (Variables|Default|GetWidgetInteractionInstance)))))))

(fn EnableCollisionwhenWalkingtoTerminal)

(fn CountMovementInputHoldTime
  (|ResetCounter)
  (Variables|Default|SetMovementInputHoldDownTimer (+ (Math|Vector|VectorLength (Class|Pawn|GetLastMovementInputVector (Game|Player|GetPlayerPawn 0))) (Variables|Default|GetMovementInputHoldDownTimer))))

(fn SaveState
  (bind _returnvalue (SaveGame|DoesSaveGameExist (Variables|Default|GetSaveSlot)))
  (if _returnvalue
    (SaveGame|DeleteGameinSlot (Variables|Default|GetSaveSlot)))
  (bind _returnvalue_2 (SaveGame|CreateSaveGameObject "/Game/WISTerminals/Blueprints/Core/BP_Terminals_SaveGame.BP_Terminals_SaveGame_C"))
  (Variables|Default|SetTerminalSaveGame _returnvalue_2)
  (bind _outactors (Actor|GetAllActorsOfClass "/Game/WISTerminals/Blueprints/Core/BP_Master_LinkedObject.BP_Master_LinkedObject_C"))
  (for _array_element _outactors
    (if (Variables|/Game/WISTerminals/Blueprints/Core/BP_Master_LinkedObject.BP_Master_LinkedObject_C|GetActive _array_element)
      (Utilities|Array|AddUnique (Variables|/Game/WISTerminals/Blueprints/Core/BP_Terminals_SaveGame.BP_Terminals_SaveGame_C|GetActivatedObjects (Variables|Default|GetTerminalSaveGame)) _array_element)))
  (Utilities|Array|Clear (Variables|/Game/WISTerminals/Blueprints/Core/BP_Terminals_SaveGame.BP_Terminals_SaveGame_C|GetUnlockedTerminals (Variables|Default|GetTerminalSaveGame)))
  (bind _outactors_2 (Actor|GetAllActorsOfClass "/Game/WISTerminals/Blueprints/BP_Computer_Terminal.BP_Computer_Terminal_C"))
  (for _array_element_2 _outactors_2
    (if (not (Variables|/Game/WISTerminals/Blueprints/Core/BP_Computer_Terminal_Master.BP_Computer_Terminal_Master_C|GetLocked _array_element_2))
      (Utilities|Array|AddUnique (Variables|/Game/WISTerminals/Blueprints/Core/BP_Terminals_SaveGame.BP_Terminals_SaveGame_C|GetUnlockedTerminals (Variables|Default|GetTerminalSaveGame)) _array_element_2)))
  (SaveGame|SaveGametoSlot (Variables|Default|GetTerminalSaveGame) (Variables|Default|GetSaveSlot)))

(fn LoadState
  (bind _returnvalue (SaveGame|DoesSaveGameExist (Variables|Default|GetSaveSlot)))
  (if _returnvalue
    (bind _returnvalue_2 (SaveGame|LoadGamefromSlot (Variables|Default|GetSaveSlot)))
    (bind _asbp_terminals_save_game (Utilities|Casting|CastToBP_Terminals_SaveGame _returnvalue_2))
    (bind _output_get (Variables|Default|SetTerminalSaveGame _asbp_terminals_save_game))
    (CallFunction|InitializeObjectStates (Variables|/Game/WISTerminals/Blueprints/Core/BP_Terminals_SaveGame.BP_Terminals_SaveGame_C|GetActivatedObjects _output_get))
    (for _array_element (Variables|/Game/WISTerminals/Blueprints/Core/BP_Terminals_SaveGame.BP_Terminals_SaveGame_C|GetUnlockedTerminals (Variables|Default|GetTerminalSaveGame))
      (Default|UnlockTerminal _array_element))))

(fn InitializeObjectStates
  (params (ActivatedObjects :type Array%20of%20BP%20Master%20Linked%20Object%20Object%20References))
  (bind _outactors (Actor|GetAllActorsOfClass "/Game/WISTerminals/Blueprints/Core/BP_Master_LinkedObject.BP_Master_LinkedObject_C"))
  (for _array_element _outactors
    (Default|Deactivate _array_element))
  (for _array_element_2 ActivatedObjects
    (Default|Activate _array_element_2))
  (bind _outactors_2 (Actor|GetAllActorsOfClass "/Game/WISTerminals/Blueprints/Core/BP_Keypad_Terminal_Master.BP_Keypad_Terminal_Master_C"))
  (for _array_element_3 _outactors_2
    (Default|InitializeKeypad _array_element_3)))